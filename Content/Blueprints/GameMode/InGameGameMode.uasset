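; InGameGameMode is the game mode for a timed soccer mini-game that tracks score, remaining time and active state.
; ResetGame respawns the ball, zeroes the score and starts a three-minute looping one-second timer, while CountdownTimer decrements time and deactivates the game at zero.
; ScoreGoal increments the score and calls SpawnBall, which destroys existing actors of a class and spawns a replacement at the soccer spawn location.
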(fn `CountdownTimer`
  (bind _gametime (`self.gameTime`))
  (if (> _gametime 0)
    (`/Engine/EditorBlueprintResources/StandardMacros.DecrementInt` _gametime)
    (else
      (set `self.gameActive` false))))

(fn `GetScore`
  (returns (score :type Integer))
  (return (`self.gameScore`)))

(fn `GetTime`
  (returns (time :type Integer))
  (return (`self.gameTime`)))

(fn `ResetGame`
  (locals (countdown :type "TimerHandle Structure"))
  (`KismetSystemLibrary.K2_ClearAndInvalidateTimerHandle` (`local.countdown`))
  (`self.SpawnBall`)
  (set `self.gameScore` 0)
  (set `self.gameTime` 180)
  (bind _returnvalue (`KismetSystemLibrary.K2_SetTimerDelegate` (`|CreateDelegate` :!event `CountdownTimer`) 1.0 true))
  (set `local.countdown` _returnvalue)
  (set `self.gameActive` true))

(fn `ScoreGoal`
  (`/Engine/EditorBlueprintResources/StandardMacros.IncrementInt` (`self.gameScore`)
    (:`  `
      (`self.SpawnBall`))))

(fn `SpawnBall`
  (bind _outactors (`GameplayStatics.GetAllActorsOfClass` null))
  (`self.K2_DestroyActor` _outactors)
  (`|SpawnActorFromClass` null (`KismetMathLibrary.Conv_VectorToTransform` (`self.soccerSpawnLocation`)) "AdjustIfPossibleButAlwaysSpawn" "OverrideRootScale" null null))

(fn `UserConstructionScript`)